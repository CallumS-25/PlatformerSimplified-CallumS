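; Platformer checkpoint actor that registers itself as LastCheckpoint on BP_ThirdPersonGameMode when the third-person character overlaps its capsule.
; Begin and end overlap share one chain, which also prints the stored checkpoint's name.
; A string Contains test on that name, with no substring supplied, chooses the ON or OFF material for this actor's cylinder only.
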(event `self.Capsule.OnComponentBeginOverlap`
  (params (OverlappedComponent :type "PrimitiveComponent Object Reference") (OtherActor :type "Actor Object Reference") (OtherComp :type "PrimitiveComponent Object Reference") (OtherBodyIndex :type Integer) (bFromSweep :type Boolean) (SweepResult :type "HitResult Structure (by ref)"))
  (bind _cylinder (`self.Cylinder`))
  (cast `/Game/ThirdPerson/Blueprints/BP_ThirdPersonCharacter` OtherActor)
  (bind _asbp_third_person_game_mode (cast `/Game/ThirdPerson/Blueprints/BP_ThirdPersonGameMode` (`GameplayStatics.GetGameMode`) :!label _label))
  (bind _output_get (set `/Game/ThirdPerson/Blueprints/BP_ThirdPersonGameMode.LastCheckpoint ` self _asbp_third_person_game_mode))
  (`KismetSystemLibrary.PrintString` (`KismetSystemLibrary.GetDisplayName` _output_get))
  (bind _asbp_third_person_game_mode_2 (cast `/Game/ThirdPerson/Blueprints/BP_ThirdPersonGameMode` (`GameplayStatics.GetGameMode`)))
  (bind _returnvalue (`KismetStringLibrary.Contains` (`KismetSystemLibrary.GetDisplayName` (`/Game/ThirdPerson/Blueprints/BP_ThirdPersonGameMode.LastCheckpoint ` _asbp_third_person_game_mode_2)) "" true))
  (if _returnvalue
    (`PrimitiveComponent.SetMaterial` _cylinder 0 "/Game/StarterContent/Materials/M_CheckpointON.M_CheckpointON")
    (elif (not _returnvalue)
      (`PrimitiveComponent.SetMaterial` _cylinder 0 "/Game/StarterContent/Materials/M_CheckpointOFF.M_CheckpointOFF"))))

(event `self.Capsule.OnComponentEndOverlap`
  (params (OverlappedComponent :type "PrimitiveComponent Object Reference") (OtherActor :type "Actor Object Reference") (OtherComp :type "PrimitiveComponent Object Reference") (OtherBodyIndex :type Integer))
  (cast `/Game/ThirdPerson/Blueprints/BP_ThirdPersonCharacter` OtherActor)
  (goto _label))

(fn `UserConstructionScript`)